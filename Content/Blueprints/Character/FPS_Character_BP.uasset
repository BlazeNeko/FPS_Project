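; First-person character Blueprint with a key binding for using an inventory item.
; Pressing L calls UseItem on the first inventory entry, then removes one item by the hard-coded name "Medicine" through the inventory component.
; An unconnected debug trace would cast 300 units forward from the camera and print the hit actor, but it never runs.
; Tick and the construction script are empty.
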(event `Key|L`
  (params (Key :type "Key Structure"))
  (bind _returnvalue (`self.GetInventoryComponent`))
  (:`Pressed`
    (bind _returnvalue_2 (`InventoryComponent.GetInventory` _returnvalue))
    (`Pickup.UseItem` (`|GetArrayItem` _returnvalue_2))
    (`InventoryComponent.RemoveFromInventory` _returnvalue "Medicine" 1)))

(event `self.ReceiveTick`
  (params (DeltaSeconds :type "Float (single-precision)")))

(fn `UserConstructionScript`)